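; Checkpoint actor that saves the player's respawn location to disk when its box component is overlapped.
; The overlap reads and prints player 0's current location, without checking which actor entered.
; It then loads the "checkpoint" save slot, or creates a Save_Respawn_BP object if none exists, stores that location as PlayerRespawnLocation and saves it back to the slot.
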(event OnComponentBeginOverlap(Box)
  (params (OverlappedComponent :type Primitive%20Component%20Object%20Reference) (OtherActor :type Actor%20Object%20Reference) (OtherComp :type Primitive%20Component%20Object%20Reference) (OtherBodyIndex :type Integer) (bFromSweep :type Boolean) (SweepResult :type Hit%20Result%20Structure%20%28by%20ref%29))
  ;[1 1 1] THis is code for capturing the locatoin of the repawn point
  (Utilities|FlowControl|Sequence
    (:then_0
      (bind _asplayer (Utilities|Casting|CastToPlayer (Game|GetPlayerCharacter 0)))
      (bind _output_get (Variables|Default|SetPlayerLocation (Transformation|GetActorLocation _asplayer)))
      (Development|PrintString (Utilities|String|ToString(Vector) _output_get)))
    (:then_1
      (bind _returnvalue (SaveGame|DoesSaveGameExist "checkpoint"))
      (if _returnvalue
        (bind _returnvalue_2 (SaveGame|LoadGamefromSlot "checkpoint"))
        (bind _assave_respawn_bp (Utilities|Casting|CastToSave_Respawn_BP _returnvalue_2))
        (Variables|/Game/Blueprints/Save_Respawn_BP.Save_Respawn_BP_C|SetPlayerRespawnLocation _assave_respawn_bp (Variables|Default|GetPlayerLocation))
        (SaveGame|SaveGametoSlot _assave_respawn_bp "checkpoint")
        (else
          (bind _returnvalue_3 (SaveGame|CreateSaveGameObject "/Game/Blueprints/Save_Respawn_BP.Save_Respawn_BP_C"))
          (Variables|/Game/Blueprints/Save_Respawn_BP.Save_Respawn_BP_C|SetPlayerRespawnLocation _returnvalue_3 (Variables|Default|GetPlayerLocation))
          (SaveGame|SaveGametoSlot _returnvalue_3 "checkpoint"))))))

(event EventBeginPlay)

(event Collision|EventActorBeginOverlap
  (params (OtherActor :type Actor%20Object%20Reference)))

(event EventTick
  (params (DeltaSeconds :type Float%20%28single-precision%29))
  ;[1 1 1] THis is code for capturing the locatoin of the repawn point
)

(fn ConstructionScript)