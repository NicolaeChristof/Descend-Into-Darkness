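; Elevator actor that the player rides or sends between points A and B with the ActivateElevator input, once TurnonElevator has powered it.
; Tick checks whether the player overlaps the control panel's Collider, enabling input and gating operation.
; Each press uses MoveComponentTo to slide ElevatorMesh to the other point and flips AtA.
; The door is shown with collision only during travel, otherwise hidden and passable.
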(event Custom|DisableDoor
  (bind _door (Variables|Default|GetDoor))
  ;[1 1 1] Door Controls
  (Rendering|SetVisibility _door false false)
  (Collision|SetCollisionEnabled _door "NoCollision"))

(event Custom|EnableDoor
  (bind _door (Variables|Default|GetDoor))
  ;[1 1 1] Door Controls
  (Rendering|SetVisibility _door true false)
  (Collision|SetCollisionEnabled _door "QueryAndPhysics"))

(event EventTick
  (params (DeltaSeconds :type Float%20%28single-precision%29))
  ;[1 1 1] Check if Player is in range of Control Pannel
  (bind _output_get (Variables|Default|SetCanOperate (Collision|IsOverlappingActor (Variables|Default|GetCollider) (Game|GetPlayerCharacter 0) :!class /Script/Engine.PrimitiveComponent)))
  (if _output_get
    (Input|EnableInput (Game|GetPlayerController 0))))

(event EventTurnonElevator
  ;[1 1 1] Turn On Elevator
  (Variables|Default|SetPowered true)
  (Development|PrintString "Elevator On"))

(event EventBeginPlay
  ;[1 1 1] Start
  (CallFunction|DisableDoor))

(event Input|ActionEvents|InputActionActivateElevator
  (params (Key :type Key%20Structure))
  ;[1 1 1] Move Elevator
  (:Pressed
    (if (Variables|Default|GetCanOperate)
      (if (Variables|Default|GetPowered)
        (if (Variables|Default|GetAtA)
          ;;[1 1 1] Move to B
          (CallFunction|EnableDoor)
          (Components|MoveComponentTo (Variables|Default|GetElevatorMesh) (.location (Transformation|GetRelativeTransform (Variables|Default|GetB))) "0, 0, 0" false false (Variables|Default|GetElevatorSpeed) false)
          (Variables|Default|SetAtA false)
          (CallFunction|DisableDoor)
          (else
            ;;[1 1 1] Move to A
            (CallFunction|EnableDoor)
            (Components|MoveComponentTo (Variables|Default|GetElevatorMesh) (.location (Transformation|GetRelativeTransform (Variables|Default|GetA))) "0, 0, 0" false false (Variables|Default|GetElevatorSpeed) false)
            (Variables|Default|SetAtA true)
            (CallFunction|DisableDoor)))))))

(fn ConstructionScript)