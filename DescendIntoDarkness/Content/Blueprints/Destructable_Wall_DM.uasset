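; Destructible wall actor that the player breaks by pressing E while in range.
; Actor overlap events set an InRange flag, and entering the overlap also enables input for the first player controller, which is never disabled on exit.
; Pressing E in range applies radius damage to the Destructible component at the actor's location.
; Tick prints InRange to the screen every frame as debug output.
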(event Collision|EventActorBeginOverlap
  (params (OtherActor :type Actor%20Object%20Reference))
  ;[1 1 1] Check if Player is in Range of Destructable Wall
  (Variables|Default|SetInRange true)
  (Input|EnableInput (Game|GetPlayerController 0)))

(event Collision|EventActorEndOverlap
  (params (OtherActor :type Actor%20Object%20Reference))
  ;[1 1 1] Check if Player is in Range of Destructable Wall
  (Variables|Default|SetInRange false))

(event EventTick
  (params (DeltaSeconds :type Float%20%28single-precision%29))
  (Development|PrintString (Utilities|String|ToString(Boolean) (Variables|Default|GetInRange))))

(event Input|KeyboardEvents|E
  (params (Key :type Key%20Structure))
  ;[1 1 1] If player presses E, Destroy Wall
  (:Pressed
    (if (Variables|Default|GetInRange)
      (Class|DestructibleComponent|ApplyRadiusDamage (Variables|Default|GetDestructible) 1.0 (Transformation|GetActorLocation) 1.0 1.0 false))))

(fn ConstructionScript)