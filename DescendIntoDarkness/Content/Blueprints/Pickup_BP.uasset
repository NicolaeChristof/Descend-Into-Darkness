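; Pickup Blueprint that shows a floating name label when the player comes close.
; The construction script fills the TextRender component from the Name variable.
; Every Tick it measures the distance between the player character and itself, showing the text within 300 units and hiding it otherwise.
; No overlap or collection logic is implemented; BeginPlay and ActorBeginOverlap are empty.
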(event EventBeginPlay)

(event Collision|EventActorBeginOverlap
  (params (OtherActor :type Actor%20Object%20Reference)))

(event EventTick
  (params (DeltaSeconds :type Float%20%28single-precision%29))
  ;[1 1 1] Show text if distance is less than 300 or hide if it's not.
  (if (< (Math|Vector|VectorLength (- (Transformation|GetActorLocation (Game|GetPlayerCharacter 0)) (Transformation|GetActorLocation))) 3e+02)
    (Rendering|SetVisibility (Variables|Default|GetTextRender) true false)
    (else
      (Rendering|SetVisibility (Variables|Default|GetTextRender) false false))))

(fn ConstructionScript
  (Rendering|Components|TextRender|SetText (Variables|Default|GetTextRender) (Utilities|Text|ToText(String) (Variables|Default|GetName))))