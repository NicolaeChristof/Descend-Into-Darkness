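; Skeleton enemy Blueprint that patrols between two points and kills the player on sight.
; From BeginPlay, GoToA and GoToB alternate AI Move To calls toward PatrolPointA and PatrolPointB, waiting DelayTime after each arrival and retrying the same leg on failure.
; PawnSensing's See Pawn event checks whether the seen pawn is player 0's character and, if so, sends it KillPlayerMessage.
; Each leg prints a debug string.
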(event OnSeePawn(PawnSensing)
  (params (Pawn :type Pawn%20Object%20Reference))
  (bind _returnvalue (Game|GetPlayerCharacter 0))
  ;[1 1 1] Kill Player upon seeing them
  (if (== Pawn _returnvalue)
    (Class|PlayerInterface|KillPlayer(Message) _returnvalue)))

(event Custom|Patrol
  ;[1 1 1] Patrol
  (CallFunction|GotoA))

(event Custom|GoToA
  ;[1 1 1] Patrol
  ;;[1 1 1] Go To A
  (Development|PrintString "Go To A" false false)
  (AI|AIMoveTo self (Transformation|GetWorldLocation (Variables|Default|GetPatrolPointA)) 0 5.0 false
    (:OnSuccess
      (Utilities|FlowControl|Delay (Variables|Default|GetDelayTime))
      (CallFunction|GotoB))
    (:OnFail
      (CallFunction|GotoA))))

(event Custom|GoToB
  ;[1 1 1] Patrol
  ;;[1 1 1] Go To B
  (Development|PrintString "Got To B")
  (AI|AIMoveTo self (Transformation|GetWorldLocation (Variables|Default|GetPatrolPointB)) 0 5.0 false
    (:OnSuccess
      (Utilities|FlowControl|Delay (Variables|Default|GetDelayTime))
      (CallFunction|GotoA))
    (:OnFail
      (CallFunction|GotoB))))

(event EventBeginPlay
  ;[1 1 1] Start
  (CallFunction|Patrol))

(fn ConstructionScript)