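; Ladder is an actor that tells the player character when it is within reach of a climbable ladder.
; On begin and end overlap it checks that the other actor is the player character, then sends it a LadderMessage with a near-ladder flag and a reference to itself.
; The ladder holds no climbing logic, and its construction script is empty.
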(event Collision|EventActorEndOverlap
  (params (OtherActor :type Actor%20Object%20Reference))
  (bind _returnvalue (Game|GetPlayerCharacter 0))
  (if (== OtherActor _returnvalue)
    (Class|PlayerInterface|Ladder(Message) _returnvalue false self)))

(event Collision|EventActorBeginOverlap
  (params (OtherActor :type Actor%20Object%20Reference))
  (bind _returnvalue (Game|GetPlayerCharacter 0))
  (if (== OtherActor _returnvalue)
    (Class|PlayerInterface|Ladder(Message) _returnvalue true self)))

(fn ConstructionScript)