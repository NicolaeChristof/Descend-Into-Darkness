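; Game mode for Descend Into Darkness that respawns the player at a saved checkpoint when the character is destroyed.
; On BeginPlay it records the player's transform, creates the "checkpoint" save if none exists, and binds to the player's destroyed event.
; On destruction it loads the saved transform, spawns and possesses a new Player, then calls Respawn to rerun that setup and rebind the event.
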(event Custom|OnDestroyed_Event_0
  (params (DestroyedActor :type Actor%20Object%20Reference))
  (bind _returnvalue (SaveGame|LoadGamefromSlot "checkpoint"))
  (bind _assave_respawn_bp (Utilities|Casting|CastToSave_Respawn_BP _returnvalue))
  (bind _output_get (Variables|Default|SetGameMode_SpawnTransform (Variables|/Game/Blueprints/Save_Respawn_BP.Save_Respawn_BP_C|GetSave_RespawnTransform _assave_respawn_bp)))
  (bind _returnvalue_2 (Game|SpawnActorfromClass "/Game/Blueprints/Player.Player_C" _output_get "Undefined" 0 0))
  (Pawn|Possess (Game|GetPlayerController 0) _returnvalue_2)
  (CallFunction|Respawn))

(event Custom|Respawn
  (Utilities|FlowControl|Sequence
    (:then_0
      ;[1 1 1] This is setting the GameMode_SpawnTransform variable equal to whatever the player's starting position is
      (bind _asplayer (Utilities|Casting|CastToPlayer (Game|GetPlayerCharacter 0)))
      (Variables|Default|SetGameMode_SpawnTransform (Transformation|GetActorTransform _asplayer)))
    (:then_1
      (bind _returnvalue (SaveGame|DoesSaveGameExist "checkpoint"))
      (if (not _returnvalue)
        (bind _returnvalue_2 (SaveGame|CreateSaveGameObject "/Game/Blueprints/Save_Respawn_BP.Save_Respawn_BP_C"))
        (Variables|/Game/Blueprints/Save_Respawn_BP.Save_Respawn_BP_C|SetSave_RespawnTransform _returnvalue_2 (Variables|Default|GetGameMode_SpawnTransform))
        (SaveGame|SaveGametoSlot _returnvalue_2 "checkpoint")
        (Development|PrintString "Made save game")))
    (:then_2
      (bind _asplayer_2 (Utilities|Casting|CastToPlayer (Game|GetPlayerCharacter 0)))
      (Game|AssignOnDestroyed _asplayer_2 (delegate Custom|OnDestroyed_Event_0)))))

(event EventBeginPlay
  (Utilities|FlowControl|Sequence
    (:then_0
      ;[1 1 1] This is setting the GameMode_SpawnTransform variable equal to whatever the player's starting position is
      (bind _asplayer (Utilities|Casting|CastToPlayer (Game|GetPlayerCharacter 0)))
      (Variables|Default|SetGameMode_SpawnTransform (Transformation|GetActorTransform _asplayer)))
    (:then_1
      (bind _returnvalue (SaveGame|DoesSaveGameExist "checkpoint"))
      (if (not _returnvalue)
        (bind _returnvalue_2 (SaveGame|CreateSaveGameObject "/Game/Blueprints/Save_Respawn_BP.Save_Respawn_BP_C"))
        (Variables|/Game/Blueprints/Save_Respawn_BP.Save_Respawn_BP_C|SetSave_RespawnTransform _returnvalue_2 (Variables|Default|GetGameMode_SpawnTransform))
        (SaveGame|SaveGametoSlot _returnvalue_2 "checkpoint")
        (Development|PrintString "Made save game")))
    (:then_2
      (bind _asplayer_2 (Utilities|Casting|CastToPlayer (Game|GetPlayerCharacter 0)))
      (Game|AssignOnDestroyed _asplayer_2 (delegate Custom|OnDestroyed_Event_0)))))

(event EventTick
  (params (DeltaSeconds :type Float%20%28single-precision%29)))

(fn ConstructionScript)