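; Side-scrolling player character, locked to X=0, with rope swinging, ledge hanging and climbing, health, fall damage and ragdoll death.
; A looping timer finds grab points by sphere trace; left mouse attaches the cable, and per-tick clamped forces drive swinging and rope climbing.
; Forward and height traces on Tick trigger ledge grabs.
; It also handles inventory UI, depth gauge spawning, ladder state and, when dead, destroying itself if a checkpoint save exists.
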(event Custom|Detach
  (bind _rope (Variables|Default|GetRope))
  (bind _charactermovement (Variables|Character|GetCharacterMovement))
  ;[1 1 1] Rope Stuff
  ;;[1 1 1] Disengage Rope
  (Variables|Default|SetAttached false)
  (Variables|/Script/CableComponent.CableComponent|SetEndLocation _rope "0, 0,30.000000")
  (Variables|/Script/CableComponent.CableComponent|SetCableGravityScale _rope 9.0)
  (Variables|/Script/CableComponent.CableComponent|SetbAttachStart _rope false)
  (Pawn|Components|CharacterMovement|SetMovementMode _charactermovement "MOVE_Falling" 0)
  (bind _retract (Timeline|Retract%20Rope PlayFromStart)
    (:Update
      (Variables|/Script/CableComponent.CableComponent|SetCableLength (Variables|Default|GetRope) _retract))
    (:Finished
      (Variables|/Script/Engine.CharacterMovementComponent|SetAirControl _charactermovement 2.0))))

(event Custom|Grab%20Ledge
  (bind _ledgenormal (Variables|Default|GetLedgeNormal))
  (bind _ledgelocation (Variables|Default|GetLedgeLocation))
  (bind _ledgenormal_2 (Variables|Default|GetLedgeNormal))
  (bind _returnvalue (Math|Conversions|RotationFromXVector _ledgenormal_2))
  (bind _returnvalue_2 (* _ledgenormal "22.000000,22.000000, 0"))
  ;[1 1 1] Edge Stuff
  ;;[1 1 1] Grab Ledge
  (if (Variables|Default|GetAttached)
    (CallFunction|Detach))
  (if (and (Variables|Default|GetWReleased) (Variables|Default|GetSReleased))
    (Class|LedgeInterface|CanGrab(Message) (Components|SkeletalMesh|GetAnimInstance (Variables|Character|GetMesh)) true)
    (Pawn|Components|CharacterMovement|SetMovementMode (Variables|Character|GetCharacterMovement) "MOVE_Flying" 0)
    (Variables|Default|SetIsLedgeHanging true)
    (Components|MoveComponentTo (Variables|Default|GetCapsuleComponent) (Math|Vector|MakeVector (+ (.x _returnvalue_2) (.x _ledgelocation)) (+ (.y _returnvalue_2) (.y _ledgelocation)) (- (.z (Variables|Default|GetLedgeHeightLocation)) 1.2e+02)) (Math|Rotator|MakeRotator (.roll _returnvalue) (.pitch _returnvalue) (- (.yaw _returnvalue) 1.8e+02)) false false 0.13 false)
    (Components|Movement|StopMovementImmediately (Variables|Character|GetCharacterMovement))))

(event Custom|Exit%20Ledge
  ;[1 1 1] Edge Stuff
  ;;[1 1 1] Exit Ledge
  (Pawn|Components|CharacterMovement|SetMovementMode (Variables|Character|GetCharacterMovement) "MOVE_Walking" 0)
  (Class|LedgeInterface|CanGrab(Message) (Components|SkeletalMesh|GetAnimInstance (Variables|Character|GetMesh)) false)
  (Variables|Default|SetIsLedgeHanging false))

(event Custom|Death
  (bind _mesh (Variables|Character|GetMesh))
  ;[1 1 1] Death
  (Variables|Default|SetAlive false)
  (Collision|SetCollisionProfileName _mesh "Ragdoll" :!class /Script/Engine.PrimitiveComponent)
  (Physics|SetSimulatePhysics _mesh true)
  (Collision|SetCollisionEnabled (Variables|Default|GetCapsuleComponent) "NoCollision")
  (Pawn|Components|CharacterMovement|DisableMovement (Variables|Character|GetCharacterMovement))
  (Development|SetHiddeninGame (Variables|Default|GetRope) true false))

(event Custom|Climb%20Up%20Ledge
  ;[1 1 1] Edge Stuff
  ;;[1 1 1] Climb Ledge
  (if (not (Variables|Default|GetIsClimbingLedge))
    (Class|LedgeInterface|ClimbLedge(Message) (Components|SkeletalMesh|GetAnimInstance (Variables|Character|GetMesh)) true)
    (Pawn|Components|CharacterMovement|SetMovementMode (Variables|Character|GetCharacterMovement) "MOVE_Flying" 0)
    (Variables|Default|SetIsClimbingLedge true)
    (Variables|Default|SetIsLedgeHanging false)))

(event Custom|Recenter%20Player
  (bind _returnvalue (Transformation|GetActorLocation))
  ;[1 1 1] Recenter player to 0 along x-axis
  (Transformation|SetActorLocation (Math|Vector|MakeVector 0.0 (.y _returnvalue) (.z _returnvalue)) false false))

(event EventBeginPlay
  ;[1 1 1] Start
  (Utilities|Time|SetTimerbyFunctionName 0 "Search Near Grab Points" 0.02 true)
  (bind _returnvalue (UserInterface|CreateWidget "/Game/Blueprints/UI/HealthUI.HealthUI_C" 0 (Variables|Default|GetCurrentHealth) (Variables|Default|GetMaxHealth)))
  (bind _output_get (Variables|Default|SetHealth _returnvalue))
  (UserInterface|Viewport|AddtoViewport _output_get 0))

(event EventTick
  (params (DeltaSeconds :type Float%20%28single-precision%29))
  ;[1 1 1] Update
  (CallFunction|RecenterPlayer)
  (CallFunction|Swing)
  (CallFunction|ForwardTracer)
  (CallFunction|HeightTracer))

(event EventClimbLedge
  (params (Is%20Climbing%20Ledge :type Boolean))
  ;[1 1 1] Edge Stuff
  ;;[1 1 1] Climb Ledge
  (Variables|Default|SetIsClimbingLedge Is%20Climbing%20Ledge)
  (Pawn|Components|CharacterMovement|SetMovementMode (Variables|Character|GetCharacterMovement) "MOVE_Walking" 0))

(event EventOnLanded
  (params (Hit :type Hit%20Result%20Structure%20%28by%20ref%29))
  (bind _charactermovement (Variables|Character|GetCharacterMovement))
  (bind _velocity (Variables|/Script/Engine.MovementComponent|GetVelocity _charactermovement))
  ;[1 1 1] Fall Damage
  ;;[1 1 1] Calculate Fall Damage
  (if (> (Variables|Default|GetCurrentHealth) 0.0)
    (if (<= (.z _velocity) (Variables|Default|GetSafeFallDistance))
      (if (<= (.z _velocity) (Variables|Default|GetInstantDeathThreshold))
        (Variables|Default|SetFallDamage (- 0.0 (Variables|Default|GetMaxHealth)))
        (else
          (Variables|Default|SetFallDamage (/ (.z _velocity) (Variables|Default|GetFallDamageMultiplier)))))
      ;;[1 1 1] Apply Damage and Update Health Bar
      (if (<= (+ (Variables|Default|GetCurrentHealth) (Variables|Default|GetFallDamage)) 0.0)
        (Variables|Default|SetCurrentHealth 0.0)
        (CallFunction|Death)
        (else
          (Variables|Default|SetCurrentHealth (+ (Variables|Default|GetCurrentHealth) (Variables|Default|GetFallDamage)))))
      (Variables|/Game/Blueprints/UI/HealthUI.HealthUI_C|SetCurrentHealth (Variables|Default|GetHealth) (Variables|Default|GetCurrentHealth))
      (else
        (Variables|Default|SetFallDamage 0.0)))))

(event EventUpdateInventoryUI
  ;[1 1 1] Update Inventory
  (Utilities|IsValid (Variables|Default|GetInventoryWidget)
    (:Is%20Valid
      (bind _foundwidgets (Widget|GetAllWidgetsOfClass "/Game/Blueprints/UI/WB_Inventory.WB_Inventory_C" true))
      (Class|InventoryWidget|LoadInventory (Utilities|Array|Get(acopy) _foundwidgets)))))

(event EventDamagePlayer
  (params (Damage :type Float%20%28single-precision%29))
  ;[1 1 1] Activates when Player is Damaged by an Enemy
  (if (<= (- (Variables|Default|GetCurrentHealth) Damage) 0.0)
    (Variables|Default|SetCurrentHealth 0.0)
    (CallFunction|Death)
    (else
      (Variables|Default|SetCurrentHealth (- (Variables|Default|GetCurrentHealth) Damage))))
  (Variables|/Game/Blueprints/UI/HealthUI.HealthUI_C|SetCurrentHealth (Variables|Default|GetHealth) (Variables|Default|GetCurrentHealth)))

(event EventKillPlayer
  ;[1 1 1] Kill Player when called by Enemy
  (bind _output_get (Variables|Default|SetCurrentHealth 0.0))
  (Variables|/Game/Blueprints/UI/HealthUI.HealthUI_C|SetCurrentHealth (Variables|Default|GetHealth) _output_get)
  (CallFunction|Death))

(event EventHealPlayer
  (params (HealthGain :type Float%20%28single-precision%29))
  (bind _maxhealth (Variables|Default|GetMaxHealth))
  ;[1 1 1] Heal Player
  (if (< (+ HealthGain (Variables|Default|GetCurrentHealth)) _maxhealth)
    (Variables|Default|SetCurrentHealth (+ HealthGain (Variables|Default|GetCurrentHealth)))
    (else
      (Variables|Default|SetCurrentHealth _maxhealth)))
  (Variables|/Game/Blueprints/UI/HealthUI.HealthUI_C|SetCurrentHealth (Variables|Default|GetHealth) (Variables|Default|GetCurrentHealth)))

(event EventLadder
  (params (NearLadder :type Boolean) (Ladder :type Ladder%20Object%20Reference))
  ;[1 1 1] Set Near Ladder Bool
  (Variables|Default|SetNearLadder NearLadder))

(event Input|ActionEvents|InputActionPrintInventory
  (params (Key :type Key%20Structure))
  ;[1 1 1] Show/Hide Inventory
  (:Pressed
    (Utilities|IsValid (Variables|Default|GetInventoryWidget)
      (:Is%20Valid
        (if (Widget|IsVisible (Variables|Default|GetInventoryWidget))
          (bind _foundwidgets (Widget|GetAllWidgetsOfClass "/Game/Blueprints/UI/WB_Inventory.WB_Inventory_C" true))
          (Widget|RemovefromParent _foundwidgets)
          (else
            (UserInterface|Viewport|AddtoViewport (Variables|Default|GetInventoryWidget) 0 :!label _label))))
      (:Is%20Not%20Valid
        (bind _returnvalue (UserInterface|CreateWidget "/Game/Blueprints/UI/WB_Inventory.WB_Inventory_C"))
        (Variables|Default|SetInventoryWidget _returnvalue)
        (goto _label)))))

(event Input|ActionEvents|InputActionPlaceCamp
  (params (Key :type Key%20Structure))
  ;[1 1 1] When the player hits the correct button when dead, the actor is destroyed (which then causes a function in BP_DescendIntoDarknessGameMode to be called)
  (:Released
    (if (not (Variables|Default|GetAlive))
      (bind _returnvalue (SaveGame|DoesSaveGameExist "checkpoint"))
      (if _returnvalue
        (Actor|DestroyActor)))))

(event Input|ActionEvents|InputActionInteractLadder
  (params (Key :type Key%20Structure))
  (:Pressed
    (if (Variables|Default|GetNearLadder)
      (bind _isa (Utilities|FlowControl|FlipFlop)
        (:A
          (Variables|Default|SetOnLadder _isa))
        (:B
          (Variables|Default|SetOnLadder _isa)))
      (else
        (Variables|Default|SetOnLadder false)))))

(event Input|AxisEvents|InputAxisMoveHorizontal
  (params (AxisValue :type Float%20%28single-precision%29))
  ;[1 1 1] Movement
  (if (not (Variables|Default|GetIsLedgeHanging))
    (Pawn|Input|AddMovementInput "0.000000,-1.000000, 0" AxisValue false)))

(event Input|MouseEvents|LeftMouseButton
  (params (Key :type Key%20Structure))
  (bind _returnvalue (Transformation|GetActorRotation))
  (bind _rope (Variables|Default|GetRope))
  (bind _grabpoint (Variables|Default|GetGrabPoint))
  (bind (_roll _pitch) (Math|Rotator|BreakRotator _returnvalue))
  ;[1 1 1] Check for Mouse Input
  (:Pressed
    (if (Variables|Default|GetAlive)
      (if (not (Variables|Default|GetIsClimbingLedge))
        (if (not (Variables|Default|GetIsLedgeHanging))
          (if (Variables|Default|GetAttached)
            (CallFunction|Detach :!label _label)
            (elif (Variables|Default|GetCanGrabAnchor)
              (bind _turn (Timeline|Turn%20Animator PlayFromStart)
                (:Update
                  ;[1 1 1] Rope Stuff
                  ;;[1 1 1] Look at Grab Point
                  (Transformation|SetActorRotation (Math|Rotator|Lerp(Rotator) _returnvalue (Math|Rotator|MakeRotator _roll _pitch (.Yaw (Math|Rotator|BreakRotator (Math|Rotator|FindLookatRotation (Transformation|GetActorLocation) (Variables|Default|GetGrabPoint))))) _turn true)))
                (:Finished
                  ;;[1 1 1] Attach Rope to Grab Point
                  (Transformation|SetWorldLocation _rope _grabpoint false false)
                  (Variables|/Script/CableComponent.CableComponent|SetbAttachStart _rope true)
                  (Variables|/Script/CableComponent.CableComponent|SetEndLocation _rope (.location (Transformation|GetSocketTransform (Variables|Character|GetMesh) "hand_rSocket" "RTS_Actor")))
                  (bind _output_get (Variables|Default|SetDistancetoGrabPoint (Math|Vector|VectorLength (- (Transformation|GetActorLocation) _grabpoint))))
                  (Variables|/Script/CableComponent.CableComponent|SetCableLength _rope (- _output_get 3e+02))
                  (Variables|Default|SetAttached true)))))))))
  (:Released
    (if (Variables|Default|GetAlive)
      (if (not (Variables|Default|GetIsLedgeHanging))
        (if (not (Variables|Default|GetIsClimbingLedge))
          (goto _label))))))

(event Input|KeyboardEvents|S
  (params (Key :type Key%20Structure))
  ;[1 1 1] Edge Stuff
  ;;[1 1 1] Exit Ledge
  (:Pressed
    (Variables|Default|SetSReleased false)
    (if (Variables|Default|GetIsLedgeHanging)
      (CallFunction|ExitLedge)))
  (:Released
    (Variables|Default|SetSReleased true)))

(event Input|KeyboardEvents|W
  (params (Key :type Key%20Structure))
  ;[1 1 1] Edge Stuff
  ;;[1 1 1] Climb Ledge
  (:Pressed
    (Variables|Default|SetWReleased false)
    (if (Variables|Default|GetIsLedgeHanging)
      (CallFunction|ClimbUpLedge)))
  (:Released
    (Variables|Default|SetWReleased true)))

(event Input|KeyboardEvents|F
  (params (Key :type Key%20Structure))
  ;[1 1 1] Spawn Depth Gauge
  (:Pressed
    (Game|SpawnActorfromClass "/Game/Blueprints/DepthGauge.DepthGauge_C" (Math|Transform|MakeTransform (+ (* (Math|Vector|GetForwardVector (Transformation|GetActorRotation)) 1e+02) (Transformation|GetActorLocation)) "0, 0, 0" "1,1,1") "Undefined" 0 (Variables|Default|GetCurrentHealth) (Variables|Default|GetSafeFallDistance) (Variables|Default|GetInstantDeathThreshold) (Variables|Default|GetFallDamageMultiplier) 0)))

(fn ConstructionScript)

(fn SearchNearGrabPoints
  (bind _returnvalue (Transformation|GetActorLocation))
  (bind _grabpoints (Variables|Default|GetGrabPoints))
  ;[1 1 1] Check for Grab Points
  (bind (_outhit _returnvalue_2) (Collision|SphereTraceByChannel _returnvalue (+ (* (Math|Vector|GetForwardVector (Transformation|GetActorRotation)) 1.0) _returnvalue) 5e+02 "TraceTypeQuery3" false 0 "None"))
  (if _returnvalue_2
    ;[1 1 1] If in Range of Grab Point
    (Utilities|Array|Add (Variables|Default|GetGrabPoints) (.HitActor (Collision|BreakHitResult _outhit)))
    (bind _asgrab_point (Utilities|Casting|CastToGrabPoint (.HitActor (Collision|BreakHitResult _outhit))))
    (if (not (Variables|Default|GetAttached))
      (Variables|Default|SetGrabPoint (Transformation|GetActorLocation _asgrab_point))
      (Rendering|SetVisibility (Variables|/Game/Blueprints/GrabPoint.GrabPoint_C|GetWidget _asgrab_point) true false)
      (Variables|Default|SetCanGrabAnchor true))
    (else
      ;[1 1 1] If Not in Range of Grab Point
      (for _array_element _grabpoints
        (bind _asgrab_point_2 (Utilities|Casting|CastToGrabPoint _array_element))
        (Rendering|SetVisibility (Variables|/Game/Blueprints/GrabPoint.GrabPoint_C|GetWidget _asgrab_point_2) false false)
        (Variables|Default|SetCanGrabAnchor false))
      (Utilities|Array|Clear _grabpoints))))

(fn Swing
  (bind _returnvalue (Transformation|GetActorLocation))
  (bind _returnvalue_2 (Input|AxisValues|GetClimbRope))
  (bind _rope (Variables|Default|GetRope))
  (bind _grabpoint (Variables|Default|GetGrabPoint))
  (bind _playergrabpointydistance (Variables|Default|GetPlayerGrabPointYDistance))
  (bind _grabpoint_2 (Variables|Default|GetGrabPoint))
  (bind _charactermovement (Variables|Character|GetCharacterMovement))
  (bind _returnvalue_3 (- _returnvalue _grabpoint_2))
  (if (Variables|Default|GetAttached)
    ;[1 1 1] Rope Update
    (Transformation|SetWorldLocation _rope (Variables|Default|GetGrabPoint) false false)
    (Variables|/Script/CableComponent.CableComponent|SetEndLocation _rope (.location (Transformation|GetSocketTransform (Variables|Character|GetMesh) "hand_rSocket" "RTS_Actor")))
    ;[1 1 1] Swing
    ;;[1 1 1] Determine Player Location in Relation to Grab Point
    (if (> (.z (Transformation|GetActorLocation)) (.z (Variables|Default|GetGrabPoint)))
      (Variables|/Script/Engine.CharacterMovementComponent|SetAirControl _charactermovement 0.0 :!label _label)
      (elif (<= (Variables|Default|GetDistancetoGrabPoint) (Variables|Default|GetMaxHangDistance))
        (Variables|/Script/Engine.CharacterMovementComponent|SetAirControl _charactermovement 1.0)
        (else
          (goto _label))))
    ;;[1 1 1] Determine Force to Apply to Player
    (Variables|Default|SetDistancetoGrabPoint (Math|Vector|VectorLength _returnvalue_3))
    ;;;[1 1 1] Calculate Climbing Force
    (if (and (or (> _returnvalue_2 0.0) (< _returnvalue_2 0.0)) (Math|Float|InRange(Float) (.y (Transformation|GetActorLocation)) (- (.y _grabpoint) _playergrabpointydistance) (+ (.y _grabpoint) _playergrabpointydistance)))
      (Variables|Default|SetClimbForce (* _returnvalue_2 2.5e+04))
      (else
        (Variables|Default|SetClimbForce (Math|Vector|DotProduct (Transformation|GetVelocity) _returnvalue_3))))
    (Physics|AddForce (Variables|Character|GetCharacterMovement) (Math|Vector|MakeVector 0.0 (Math|Float|Clamp(Float) (.y (* (* (Math|Vector|Normalize _returnvalue_3) (Variables|Default|GetClimbForce)) -12.0)) (Variables|Default|GetMinYClamp) (Variables|Default|GetMaxYClamp)) (Math|Float|Clamp(Float) (.z (* (* (Math|Vector|Normalize _returnvalue_3) (Variables|Default|GetClimbForce)) -12.0)) (Variables|Default|GetMinZClamp) (Variables|Default|GetMaxZClamp))))
    (Development|PrintString (Utilities|String|ToString(Float) (Variables|Default|GetDistancetoGrabPoint)) false false "(R=0.000000,G=0.660000,B=1.000000,A=1.000000)" 1e+01)
    ;[1 1 1] Set Air Parameters
    (Variables|/Script/CableComponent.CableComponent|SetCableLength (Variables|Default|GetRope) (- (Variables|Default|GetDistancetoGrabPoint) 3e+02))))

(fn ForwardTracer
  (bind _returnvalue (Transformation|GetActorLocation))
  (bind _returnvalue_2 (Transformation|GetActorRotation))
  (bind _returnvalue_3 (Math|Vector|GetForwardVector _returnvalue_2))
  ;[1 1 1] Check for Grabable Ledges
  (bind (_outhit _returnvalue_4) (Collision|SphereTraceByChannel _returnvalue (+ (Math|Vector|MakeVector (* (.x _returnvalue_3) 1.5e+02) (* (.y _returnvalue_3) 1.5e+02) (.z _returnvalue_3)) _returnvalue) 2e+01 "TraceTypeQuery4" false (Utilities|Array|MakeArray 0) "None"))
  (if _returnvalue_4
    (Variables|Default|SetLedgeLocation (.Location (Collision|BreakHitResult _outhit)))
    (Variables|Default|SetLedgeNormal (.Normal (Collision|BreakHitResult _outhit)))))

(fn HeightTracer
  (bind _returnvalue (Transformation|GetActorLocation))
  (bind _returnvalue_2 (Transformation|GetActorRotation))
  (bind (_x _y _z) (Math|Vector|BreakVector _returnvalue))
  (bind _returnvalue_3 (Math|Vector|GetForwardVector _returnvalue_2))
  (bind _returnvalue_4 (* _returnvalue_3 7e+01))
  (bind _returnvalue_5 (+ _z 5e+02))
  (bind _returnvalue_6 (Math|Vector|MakeVector _x _y _returnvalue_5))
  (bind _returnvalue_7 (+ _returnvalue_6 _returnvalue_4))
  (bind (_x_2 _y_2 _z_2) (Math|Vector|BreakVector _returnvalue_7))
  ;[1 1 1] Check for Grabable Ledges
  (bind (_outhit _returnvalue_8) (Collision|SphereTraceByChannel _returnvalue_7 (Math|Vector|MakeVector _x_2 _y_2 (- _z_2 5e+02)) 2e+01 "TraceTypeQuery4" false (Utilities|Array|MakeArray 0) "None"))
  (if _returnvalue_8
    ;[1 1 1] Check if Player Hip is within Range of Ledge
    (Variables|Default|SetLedgeHeightLocation (.Location (Collision|BreakHitResult _outhit)))
    (if (Math|Float|InRange(Float) (- (.z (Transformation|GetSocketLocation (Variables|Character|GetMesh) (Variables|Default|GetPelvisSocket))) (.z (Variables|Default|GetLedgeHeightLocation))) -5e+01 0.0)
      (if (not (Variables|Default|GetIsClimbingLedge))
        (CallFunction|GrabLedge)))))