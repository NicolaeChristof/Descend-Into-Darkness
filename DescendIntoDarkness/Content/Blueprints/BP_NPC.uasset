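; NPC Blueprint that shows and clears its dialogue on screen through the WB_Dialogue widget.
; UpdateDialogue removes top-level dialogue widgets, then creates a fresh one filled with the NPC's CurrentLine and Name and adds it to the viewport.
; ClearDialogue only removes those widgets; nothing in this graph triggers either event or sets the line.
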(event EventBeginPlay)

(event Collision|EventActorBeginOverlap
  (params (OtherActor :type Actor%20Object%20Reference)))

(event EventUpdateDialogue
  ;[1 1 1] Update Line
  (bind _foundwidgets (Widget|GetAllWidgetsOfClass "/Game/Blueprints/Dialogue/WB_Dialogue.WB_Dialogue_C" true))
  (Widget|RemovefromParent _foundwidgets)
  (bind _returnvalue (UserInterface|CreateWidget "/Game/Blueprints/Dialogue/WB_Dialogue.WB_Dialogue_C"))
  (Variables|/Game/Blueprints/Dialogue/WB_Dialogue.WB_Dialogue_C|SetDialogueText _returnvalue (Variables|Default|GetCurrentLine))
  (Variables|/Game/Blueprints/Dialogue/WB_Dialogue.WB_Dialogue_C|SetNameText _returnvalue (Utilities|Text|ToText(Name) (Variables|Default|GetName)))
  (UserInterface|Viewport|AddtoViewport _returnvalue 0))

(event EventClearDialogue
  ;[1 1 1] Clear Dialogue
  (bind _foundwidgets (Widget|GetAllWidgetsOfClass "/Game/Blueprints/Dialogue/WB_Dialogue.WB_Dialogue_C" true))
  (Widget|RemovefromParent _foundwidgets))

(fn ConstructionScript)