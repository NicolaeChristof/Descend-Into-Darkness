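; Destructible floor actor that the player can break with the ShovelPick input while inside its collider.
; Tick checks the player's overlap and enables input while in range, with no matching disable, so the press handler rechecks the range flag.
; A press applies radius damage from the player's location to the Destructible component, then after short delays makes it ignore Pawn collision and later destroys the actor.
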(event EventTick
  (params (DeltaSeconds :type Float%20%28single-precision%29))
  ;[1 1 1] Check if Player is in Range of Destructible Wall
  (bind _output_get (Variables|Default|SetInRange (Collision|IsOverlappingActor (Variables|Default|GetCollider) (Game|GetPlayerCharacter 0) :!class /Script/Engine.PrimitiveComponent)))
  (if _output_get
    (Input|EnableInput (Game|GetPlayerController 0))))

(event Input|ActionEvents|InputActionShovelPick
  (params (Key :type Key%20Structure))
  (bind _destructible (Variables|Default|GetDestructible))
  ;[1 1 1] If player presses E, Destroy Floor
  (:Pressed
    (if (Variables|Default|GetInRange)
      (Class|DestructibleComponent|ApplyRadiusDamage _destructible 1e+02 (Transformation|GetActorLocation (Game|GetPlayerCharacter 0)) 1e+02 1e+02 false)
      (Utilities|FlowControl|Delay 0.2)
      (Collision|SetCollisionResponsetoChannel _destructible "ECC_Pawn" "ECR_Ignore")
      (Utilities|FlowControl|Delay 5.0)
      (Actor|DestroyActor))))

(fn ConstructionScript)