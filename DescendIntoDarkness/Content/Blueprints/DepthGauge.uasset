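; DepthGauge is a physics-driven sphere actor that judges whether it survives an impact from its fall speed.
; BeginPlay enables physics simulation and gravity on the sphere.
; On hit, vertical velocity sets a Survive flag false at or below the instant-death threshold, true at or above the safe limit, and leaves it unchanged between.
; Actor destruction and the fall-damage multiplier calculation are not connected.
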(event EventBeginPlay
  (bind _sphere (Variables|Default|GetSphere))
  (Physics|SetSimulatePhysics _sphere true)
  (Physics|SetEnableGravity _sphere true))

(event Collision|EventActorBeginOverlap
  (params (OtherActor :type Actor%20Object%20Reference)))

(event EventTick
  (params (DeltaSeconds :type Float%20%28single-precision%29)))

(event Collision|EventHit
  (params (MyComp :type Primitive%20Component%20Object%20Reference) (Other :type Actor%20Object%20Reference) (OtherComp :type Primitive%20Component%20Object%20Reference) (bSelfMoved :type Boolean) (HitLocation :type Vector :default "0, 0, 0") (HitNormal :type Vector :default "0, 0, 0") (NormalImpulse :type Vector :default "0, 0, 0") (Hit :type Hit%20Result%20Structure%20%28by%20ref%29))
  (bind _returnvalue (Transformation|GetVelocity))
  (if (< (.z _returnvalue) (Variables|Default|GetSafeFallDistance))
    (if (<= (.z _returnvalue) (Variables|Default|GetInstantDeathThreshold))
      (Variables|Default|SetSurvive false))
    (else
      (Variables|Default|SetSurvive true))))

(fn ConstructionScript)