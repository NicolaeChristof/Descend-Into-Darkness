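; LockedDoor is a door actor that the player opens with a matching key.
; Each Tick stores whether the player overlaps its Collider and enables input while they do, with no matching disable.
; Pressing OpenDoor in range sends CheckForKeyMessage to the player character with the DoorID and a self reference.
; The HasKey event receives the result and destroys the door when true.
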(event EventTick
  (params (DeltaSeconds :type Float%20%28single-precision%29))
  ;[1 1 1] Check if Player is in Range of Door
  (bind _output_get (Variables|Default|SetInRange (Collision|IsOverlappingActor (Variables|Default|GetCollider) (Game|GetPlayerCharacter 0) :!class /Script/Engine.PrimitiveComponent)))
  (if _output_get
    (Input|EnableInput (Game|GetPlayerController 0))))

(event EventHasKey
  (params (HasKey :type Boolean))
  ;[1 1 1] If the Player has the Key, Open the Door
  (if HasKey
    (Actor|DestroyActor)))

(event Input|ActionEvents|InputActionOpenDoor
  (params (Key :type Key%20Structure))
  ;[1 1 1] Check if Player has a Matching Key for this Door
  (:Pressed
    (if (Variables|Default|GetInRange)
      (Class|PlayerInterface|CheckforKey(Message) (Game|GetPlayerCharacter 0) (Variables|Default|GetDoorID) self))))

(fn ConstructionScript)